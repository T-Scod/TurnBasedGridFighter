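; Player controller for a two-player, turn-based grid tactics game, handling camera input, cell selection, combat and turns.
; Clicks select characters, flagging move and attack cells by repeatedly expanding cell neighbours, then issue AI MoveTo orders.
; Tick resolves pending attacks once movement is idle, applying damage, deaths and the win check.
; Each move or attack consumes one of the player's per-character moves; at zero, the turn passes.
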(event Custom|TurnChange
  ;[1 1 1] Resets the turn specific values and changes the player index
  (bind _output_get (Variables|Default|SetPlayerIndexTurn (Utilities|Select :Index (Variables|Default|GetPlayerIndexTurn) :Option%200 1 :Option%201 0)))
  (Variables|Default|SetRemainingMoves (Utilities|Array|Get(acopy) (Variables|Default|GetCharacterAmount) _output_get))
  (Default|TurnChange (Variables|Default|GetMainHUD) (Variables|Default|GetPlayerIndexTurn))
  (for _array_element (Variables|Default|GetAllCharacters)
    (Variables|/Game/Characters/BP_CharacterBase.BP_CharacterBase_C|SetHasMoved _array_element false)))

(event Custom|ConsumeTurn
  ;[1 1 1] Reduces the number of remaining moves and changes turns if needed
  (bind _output_get (Variables|Default|SetRemainingMoves (- (Variables|Default|GetRemainingMoves) 1)))
  (if (== _output_get 0)
    (CallFunction|TurnChange)))

(event EventBeginPlay
  (bind _characteramount (Variables|Default|GetCharacterAmount))
  (bind _characteramount_2 (Variables|Default|GetCharacterAmount))
  ;[1 1 1] Initialise the player pawn, cursor, grid manager and characters
  (bind _asbp_camera_pawn (Utilities|Casting|CastToBP_CameraPawn (Game|Player|GetPlayerPawn 0)))
  (Variables|Default|SetCameraPawn _asbp_camera_pawn)
  (Utilities|FlowControl|Delay 0.2)
  (bind _foundwidgets (Widget|GetAllWidgetsOfClass "/Game/Widgets/W_MainHUD.W_MainHUD_C" true))
  (Variables|Default|SetMainHUD (Utilities|Array|Get(acopy) _foundwidgets))
  (bind _returnvalue (Actor|GetActorOfClass "/Game/Blueprints/BP_Cursor.BP_Cursor_C"))
  (Variables|Default|SetCursor _returnvalue)
  (bind _returnvalue_2 (Actor|GetActorOfClass "/Game/Blueprints/BP_GridManager.BP_GridManager_C"))
  (Variables|Default|SetGridManager _returnvalue_2)
  (Utilities|Array|Add _characteramount 0)
  (Utilities|Array|Add _characteramount 0)
  (bind _outactors (Actor|GetAllActorsOfClass "/Game/Characters/BP_CharacterBase.BP_CharacterBase_C"))
  (bind _output_get (Variables|Default|SetAllCharacters _outactors))
  (for _array_element _output_get
    (Utilities|Array|SetArrayElem _characteramount_2 (Variables|/Game/Characters/BP_CharacterBase.BP_CharacterBase_C|GetPlayerIndex _array_element) (+ (Utilities|Array|Get(acopy) _characteramount_2 (Variables|/Game/Characters/BP_CharacterBase.BP_CharacterBase_C|GetPlayerIndex _array_element)) 1)))
  (Variables|Default|SetRemainingMoves (Utilities|Array|Get(acopy) (Variables|Default|GetCharacterAmount) (Variables|Default|GetPlayerIndexTurn))))

(event EventTick
  (params (DeltaSeconds :type Float%20%28single-precision%29))
  (bind _characteramount (Variables|Default|GetCharacterAmount))
  (bind _playerindexturn (Variables|Default|GetPlayerIndexTurn))
  (bind _returnvalue (Utilities|Select :Index _playerindexturn :Option%200 1 :Option%201 0))
  ;[1 1 1] Check if the character should be attacking
  (bind _selectedcharacter (Variables|Default|GetSelectedCharacter)
    (:then
      (if (and (Variables|Default|GetIsAttacking) (Utilities|Enum|Equal(Enum) (Class|AIController|GetMoveStatus (AI|GetAIController _selectedcharacter)) "Idle"))
        (Variables|/Game/Characters/BP_CharacterBase.BP_CharacterBase_C|SetHasMoved _selectedcharacter true)
        (Default|AttackAnimation _selectedcharacter)
        ;[1 1 1] Damages the opponent
        (Default|KnockbackAnimation (Variables|Default|GetOpposingCharacter))
        (Variables|Default|SetIsAttacking false)
        (bind _output_get (Variables|/Game/Characters/BP_CharacterBase.BP_CharacterBase_C|SetHealth (Variables|Default|GetOpposingCharacter) (- (Variables|/Game/Characters/BP_CharacterBase.BP_CharacterBase_C|GetHealth (Variables|Default|GetOpposingCharacter)) (Variables|/Game/Characters/BP_CharacterBase.BP_CharacterBase_C|GetAttack (Variables|Default|GetSelectedCharacter)))))
        (if (<= _output_get 0)
          (Variables|/Game/Characters/BP_CharacterBase.BP_CharacterBase_C|SetIsDead (Variables|Default|GetOpposingCharacter) true)
          (Utilities|Array|RemoveItem (Variables|Default|GetAllCharacters) (Variables|Default|GetOpposingCharacter))
          (Default|Die (Variables|Default|GetOpposingCharacter))
          ;[1 1 1] Removes the opponent if they are dead and updates the win condition
          (Utilities|Array|SetArrayElem _characteramount _returnvalue (- (Utilities|Array|Get(acopy) _characteramount _returnvalue) 1)))
        (Variables|Default|SetSelectedCharacter 0)
        (Variables|Default|SetOpposingCharacter 0)
        (if (== (Utilities|Array|Get(acopy) (Variables|Default|GetCharacterAmount) (Utilities|Select :Index (Variables|Default|GetPlayerIndexTurn) :Option%200 1 :Option%201 0)) 0)
          (Default|WinScreen (Variables|Default|GetMainHUD) (Variables|Default|GetPlayerIndexTurn))
          (else
            (CallFunction|ConsumeTurn)))))
    (:else)))

(event Input|ActionEvents|InputActionZoomIn
  (params (Key :type Key%20Structure :default "None"))
  ;[1 1 1] User movement input
  (:Pressed
    (Default|Zoom (Variables|Default|GetCameraPawn) -1.0)))

(event Input|ActionEvents|InputActionZoomOut
  (params (Key :type Key%20Structure :default "None"))
  ;[1 1 1] User movement input
  (:Pressed
    (Default|Zoom (Variables|Default|GetCameraPawn) 1.0)))

(event Input|AxisEvents|InputAxisMoveForward
  (params (AxisValue :type Float%20%28single-precision%29))
  ;[1 1 1] User movement input
  (Default|MoveForward (Variables|Default|GetCameraPawn) AxisValue))

(event Input|AxisEvents|InputAxisMoveRight
  (params (AxisValue :type Float%20%28single-precision%29))
  ;[1 1 1] User movement input
  (Default|MoveRight (Variables|Default|GetCameraPawn) AxisValue))

(event Input|MouseEvents|LeftMouseButton
  (params (Key :type Key%20Structure :default "None"))
  ;[1 1 1] Selects a grid cell and runs the logic for it. Does not operate while a character is moving
  (:Pressed
    (bind _selectedcharacter (Variables|Default|GetSelectedCharacter)
      (:then
        (if (Utilities|Enum|Equal(Enum) (Class|AIController|GetMoveStatus (AI|GetAIController _selectedcharacter)) "Idle")
          (Variables|Default|SetSelectedCharacter 0)
          (CallFunction|SelectGridCell :!label _label)))
      (:else
        (goto _label)))))

(fn ConstructionScript)

(fn AddNeighbours
  (params (GridCell :type BP%20Grid%20Cell%20Object%20Reference))
  ;[1 1 1] Gets all the available cells around the given cell
  (bind _neighbours (Default|GetNeighboursasArray GridCell))
  (for _array_element _neighbours
    (Utilities|IsValid _array_element
      (:Is%20Valid
        (Variables|/Game/Blueprints/BP_GridCell.BP_GridCell_C|SetAvailable _array_element true)
        (Utilities|Set|Add (Variables|Default|GetNeighbourCells) _array_element)
        (bind _characterref (Variables|/Game/Blueprints/BP_GridCell.BP_GridCell_C|GetCharacterRef _array_element)
          (:then
            (if (!= (Variables|/Game/Characters/BP_CharacterBase.BP_CharacterBase_C|GetPlayerIndex (Variables|/Game/Blueprints/BP_GridCell.BP_GridCell_C|GetCharacterRef (Variables|/Game/Blueprints/BP_Cursor.BP_Cursor_C|GetGridCell (Variables|Default|GetCursor)))) (Variables|/Game/Characters/BP_CharacterBase.BP_CharacterBase_C|GetPlayerIndex _characterref))
              (Rendering|Material|SetMaterial (Variables|/Game/Blueprints/BP_GridCell.BP_GridCell_C|GetPlane _array_element) 0 "/Game/Materials/M_Attackable.M_Attackable")
              (else
                (Rendering|Material|SetMaterial (Variables|/Game/Blueprints/BP_GridCell.BP_GridCell_C|GetPlane _array_element) 0 "/Game/Materials/M_Available.M_Available" :!label _label))))
          (:else
            (goto _label)))))))

(fn SelectGridCell
  (bind _cursor (Variables|Default|GetCursor))
  (bind _cursor_2 (Variables|Default|GetCursor))
  (bind _gridcell (Variables|/Game/Blueprints/BP_Cursor.BP_Cursor_C|GetGridCell _cursor_2))
  (bind _gridcell_2 (Variables|/Game/Blueprints/BP_Cursor.BP_Cursor_C|GetGridCell _cursor))
  (bind _gridcell_3 (Variables|/Game/Blueprints/BP_Cursor.BP_Cursor_C|GetGridCell (Variables|Default|GetCursor))
    (:then
      (bind _characterref (Variables|/Game/Blueprints/BP_GridCell.BP_GridCell_C|GetCharacterRef _gridcell_3)
        (:then
          ;[1 1 1] Selects a character and displays their movement and attack range
          (if (== (Variables|Default|GetPlayerIndexTurn) (Variables|/Game/Characters/BP_CharacterBase.BP_CharacterBase_C|GetPlayerIndex _characterref))
            (CallFunction|ClearSelection :!label _label)
            (CallFunction|AddNeighbours _gridcell_2)
            (Utilities|Set|Add (Variables|Default|GetNeighbourCells) _gridcell_2)
            (Variables|/Game/Blueprints/BP_GridCell.BP_GridCell_C|SetAvailable _gridcell_2 true)
            (for _index (range 1 (- (Variables|/Game/Characters/BP_CharacterBase.BP_CharacterBase_C|GetMovement (Variables|/Game/Blueprints/BP_GridCell.BP_GridCell_C|GetCharacterRef _gridcell_2)) 1))
              (bind _result (Utilities|Set|ToArray (Variables|Default|GetNeighbourCells)))
              (for _array_element _result
                (CallFunction|AddNeighbours _array_element)))
            (for _index_2 (range 1 (Variables|/Game/Characters/BP_CharacterBase.BP_CharacterBase_C|GetRange (Variables|/Game/Blueprints/BP_GridCell.BP_GridCell_C|GetCharacterRef _gridcell_2)))
              (bind _result_2 (Utilities|Set|ToArray (Variables|Default|GetNeighbourCells)))
              (for _array_element_2 _result_2
                (CallFunction|AddAttackRange _array_element_2)))
            (bind _output_get (Variables|Default|SetSelectedGridCell (Variables|/Game/Blueprints/BP_Cursor.BP_Cursor_C|GetGridCell (Variables|Default|GetCursor))))
            (Rendering|Material|SetMaterial (Variables|/Game/Blueprints/BP_GridCell.BP_GridCell_C|GetPlane _output_get) 0 "/Game/Materials/M_Available.M_Available")
            (else
              ;[1 1 1] Moves the selected character to an opponent and starts attacking
              (bind _selectedgridcell (Variables|Default|GetSelectedGridCell)
                (:then
                  (bind _characterref_2 (Variables|/Game/Blueprints/BP_GridCell.BP_GridCell_C|GetCharacterRef _selectedgridcell)
                    (:then
                      (if (not (Variables|/Game/Characters/BP_CharacterBase.BP_CharacterBase_C|GetHasMoved _characterref_2))
                        (if (== (Variables|/Game/Characters/BP_CharacterBase.BP_CharacterBase_C|GetPlayerIndex _characterref_2) (Variables|Default|GetPlayerIndexTurn))
                          (if (Variables|/Game/Blueprints/BP_GridCell.BP_GridCell_C|GetAvailable _gridcell)
                            (bind _gridcell_4 (Default|CalculateAttackableGridCells (Variables|Default|GetGridManager) _gridcell (Variables|Default|GetSelectedGridCell)))
                            (Utilities|IsValid _gridcell_4
                              (:Is%20Valid
                                (Variables|Default|SetSelectedCharacter _characterref_2)
                                (AI|Navigation|MovetoLocation (AI|GetAIController _characterref_2) (Transformation|GetActorLocation _gridcell_4) -1.0 true true false true 0 false)
                                (Variables|Default|SetIsAttacking true)
                                (CallFunction|ClearSelection)
                                (Variables|/Game/Blueprints/BP_GridCell.BP_GridCell_C|SetCharacterRef (Variables|Default|GetSelectedGridCell) 0)
                                (Variables|Default|SetOpposingCharacter (Variables|/Game/Blueprints/BP_GridCell.BP_GridCell_C|GetCharacterRef _gridcell))
                                (Variables|/Game/Blueprints/BP_GridCell.BP_GridCell_C|SetCharacterRef _gridcell_4 (Variables|Default|GetSelectedCharacter))
                                (Variables|Default|SetSelectedGridCell 0)))
                            (else
                              (goto _label)))
                          (else
                            (goto _label)))))
                    (:else
                      (goto _label))))
                (:else
                  (goto _label))))))
        (:else
          ;[1 1 1] Moves a character to the selected cell
          (bind _selectedgridcell_2 (Variables|Default|GetSelectedGridCell)
            (:then
              (bind _characterref_3 (Variables|/Game/Blueprints/BP_GridCell.BP_GridCell_C|GetCharacterRef _selectedgridcell_2)
                (:then
                  (if (Math|Boolean|ANDBoolean (== (Variables|/Game/Characters/BP_CharacterBase.BP_CharacterBase_C|GetPlayerIndex _characterref_3) (Variables|Default|GetPlayerIndexTurn)) (not (Variables|/Game/Characters/BP_CharacterBase.BP_CharacterBase_C|GetHasMoved _characterref_3)) (Variables|/Game/Blueprints/BP_GridCell.BP_GridCell_C|GetAvailable _gridcell_3) (== (Rendering|Material|GetMaterial (Variables|/Game/Blueprints/BP_GridCell.BP_GridCell_C|GetPlane _gridcell_3) 0) "/Game/Materials/M_Available.M_Available"))
                    (bind _output_get_2 (Variables|/Game/Blueprints/BP_GridCell.BP_GridCell_C|SetCharacterRef _gridcell_3 _characterref_3))
                    (bind _output_get_3 (Variables|Default|SetSelectedCharacter _output_get_2))
                    (Variables|/Game/Characters/BP_CharacterBase.BP_CharacterBase_C|SetHasMoved _output_get_3 true)
                    (AI|Navigation|MovetoLocation (AI|GetAIController _characterref_3) (Transformation|GetActorLocation _gridcell_3) -1.0 true true false true 0)
                    (Variables|/Game/Blueprints/BP_GridCell.BP_GridCell_C|SetCharacterRef (Variables|Default|GetSelectedGridCell) 0)
                    (CallFunction|ClearSelection)
                    (Variables|Default|SetSelectedGridCell 0)
                    (CallFunction|ConsumeTurn)
                    (else
                      (CallFunction|ClearSelection :!label _label_2)
                      (Rendering|Material|SetMaterial (Variables|/Game/Blueprints/BP_GridCell.BP_GridCell_C|GetPlane _gridcell_3) 0 "/Game/Materials/M_Selected.M_Selected")
                      (Variables|Default|SetSelectedGridCell _gridcell_3))))
                (:else
                  (goto _label_2))))
            (:else
              (goto _label_2))))))
    (:else)))

(fn ClearSelection
  ;[1 1 1] Clears all of the available cells
  (bind _selectedgridcell (Variables|Default|GetSelectedGridCell)
    (:then
      (Rendering|Material|SetMaterial (Variables|/Game/Blueprints/BP_GridCell.BP_GridCell_C|GetPlane _selectedgridcell) 0 "/Game/Materials/M_Unselected.M_Unselected")
      (bind _result (Utilities|Set|ToArray (Variables|Default|GetNeighbourCells)))
      (for _array_element _result
        (Variables|/Game/Blueprints/BP_GridCell.BP_GridCell_C|SetAvailable _array_element false)
        (Rendering|Material|SetMaterial (Variables|/Game/Blueprints/BP_GridCell.BP_GridCell_C|GetPlane _array_element) 0 "/Game/Materials/M_Unselected.M_Unselected"))
      (Utilities|Set|Clear (Variables|Default|GetNeighbourCells))
      (return))
    (:else)))

(fn AddAttackRange
  (params (GridCell :type BP%20Grid%20Cell%20Object%20Reference))
  ;[1 1 1] Adds the attack range to the available cells
  (bind _neighbours (Default|GetNeighboursasArray GridCell))
  (for _array_element _neighbours
    (Utilities|IsValid _array_element
      (:Is%20Valid
        (if (not (Variables|/Game/Blueprints/BP_GridCell.BP_GridCell_C|GetAvailable _array_element))
          (Variables|/Game/Blueprints/BP_GridCell.BP_GridCell_C|SetAvailable _array_element true)
          (Utilities|Set|Add (Variables|Default|GetNeighbourCells) _array_element)
          (Rendering|Material|SetMaterial (Variables|/Game/Blueprints/BP_GridCell.BP_GridCell_C|GetPlane _array_element) 0 "/Game/Materials/M_Attackable.M_Attackable"))))))