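; BP_CameraPawn is a player-movable camera pawn with spring-arm zoom and bounded panning.
; Zoom input changes the arm length within min/max limits, then OnZoomChange scales FloatingPawnMovement's max speed from its starting value in proportion to zoom distance.
; Forward and right inputs add movement along actor vectors only while world Y and X respectively stay within limits, assuming a fixed orientation where negative right input increases X.
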(event Custom|MoveRight
  (params (Magnitude :type Float%20%28double-precision%29))
  (bind _returnvalue (Transformation|GetActorLocation))
  ;[1 1 1] Move right and left
  (if (< Magnitude 0.0)
    (if (< (.x _returnvalue) (Variables|Default|GetMaxX))
      (Pawn|Input|AddMovementInput (Transformation|GetActorRightVector) (* Magnitude (Variables|Default|GetMoveSpeed)) false :!label _label))
    (elif (> (.x _returnvalue) (Variables|Default|GetMinX))
      (goto _label))))

(event Custom|Zoom
  (params (InputScale :type Float%20%28double-precision%29))
  (bind _springarm (Variables|Default|GetSpringArm))
  ;[1 1 1] Zoom in and out
  (Variables|/Script/Engine.SpringArmComponent|SetTargetArmLength _springarm (Math|Float|Clamp(Float) (+ (* InputScale (Variables|Default|GetZoomSpeed)) (Variables|/Script/Engine.SpringArmComponent|GetTargetArmLength _springarm)) (Variables|Default|GetMinZoom) (Variables|Default|GetMaxZoom)))
  (CallFunction|OnZoomChange))

(event Custom|MoveForward
  (params (Magnitude :type Float%20%28double-precision%29))
  (bind _returnvalue (Transformation|GetActorLocation))
  ;[1 1 1] Move forward and back
  (if (> Magnitude 0.0)
    (if (< (.y _returnvalue) (Variables|Default|GetMaxY))
      (Pawn|Input|AddMovementInput (Transformation|GetActorForwardVector) (* Magnitude (Variables|Default|GetMoveSpeed)) false :!label _label))
    (elif (> (.y _returnvalue) (Variables|Default|GetMinY))
      (goto _label))))

(event EventBeginPlay
  ;[1 1 1] Initialise move speed
  (Variables|Default|SetInitialMoveSpeed (Class|MovementComponent|GetMaxSpeed (Variables|Default|GetFloatingPawnMovement)))
  (CallFunction|OnZoomChange))

(fn ConstructionScript)

(fn OnZoomChange
  ;[1 1 1] Changes the move speed based on the zoom amount
  (Variables|/Script/Engine.FloatingPawnMovement|SetMaxSpeed (Variables|Default|GetFloatingPawnMovement) (* (Variables|Default|GetInitialMoveSpeed) (/ (Variables|/Script/Engine.SpringArmComponent|GetTargetArmLength (Variables|Default|GetSpringArm)) (Variables|Default|GetMinZoom)))))