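; BP_Cursor is an actor that follows the mouse across the game's grid, snapping to the cell under the pointer.
; On BeginPlay it caches the grid manager and player controller.
; Every tick it deprojects the mouse position into a Camera-channel line trace, asks the grid manager for the cell closest to the hit, stores it and moves to that cell's location.
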(event EventBeginPlay
  ;[1 1 1] Initialises the grid manager and player controller references
  (bind _returnvalue (Actor|GetActorOfClass "/Game/Blueprints/BP_GridManager.BP_GridManager_C"))
  (Variables|Default|SetGridManager _returnvalue)
  (bind _asbp_player_controller (Utilities|Casting|CastToBP_PlayerController (Game|GetPlayerController 0)))
  (Variables|Default|SetPlayerController _asbp_player_controller))

(event EventTick
  (params (DeltaSeconds :type Float%20%28single-precision%29))
  (CallFunction|UpdateCursorPos))

(fn ConstructionScript)

(fn UpdateCursorPos
  (bind _playercontroller (Variables|Default|GetPlayerController))
  (bind (_worldlocation _worlddirection) (Game|Player|ConvertMouseLocationToWorldSpace _playercontroller))
  ;[1 1 1] Updates the location of the cursor based on the mouse pos
  (bind _outhit (Collision|LineTraceByChannel _worldlocation (+ _worldlocation (* _worlddirection 1e+04)) "TraceTypeQuery2" false 0 "None"))
  (if (.bBlockingHit (Collision|BreakHitResult _outhit))
    (bind _gridcell (Default|GetClosestGridCell (Variables|Default|GetGridManager) (.Location (Collision|BreakHitResult _outhit))))
    (bind _output_get (Variables|Default|SetGridCell _gridcell))
    (Transformation|SetActorLocation (Transformation|GetActorLocation _output_get) false false)))